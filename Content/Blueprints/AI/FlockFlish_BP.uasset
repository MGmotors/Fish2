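; A single boid fish in a flock that can be eaten, which hides it and disables its collision until a timer restores it.
; Each tick it eases its heading toward a target, moves in 2D pane coordinates with clamped height, then maps to world space through the flock's Pane.
; The target refreshes at random ticks from weighted cohesion, alignment, separation and goal-seeking vectors computed over the Flock's fish.
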(event `Recovered`
  (`SceneComponent.SetHiddenInGame` (`self.DefaultSceneRoot`) false true)
  (`PrimitiveComponent.SetCollisionEnabled` (`self.Capsule`) "QueryAndPhysics"))

(event `Eaten`
  (`SceneComponent.SetHiddenInGame` (`self.DefaultSceneRoot`) true true)
  (`PrimitiveComponent.SetCollisionEnabled` (`self.Capsule`) "NoCollision")
  (`KismetSystemLibrary.K2_SetTimer` self "Recovered" 6.0))

(event `self.ReceiveTick`
  (params (DeltaSeconds :type "Float (single-precision)"))
  (`self.updateDirection` DeltaSeconds)
  (`self.updateLocation` DeltaSeconds)
  (`self.updateTargetDirection`))

(fn `calcAvgDirection`
  (params (Fishes :type "Array of /Game/Blueprints/AI/FlockFlish_BP Object Reference"))
  (returns (avgDirection :type "Vector2D Structure"))
  (locals (accumulatedDirection :type "Vector2D Structure"))
  (for _array_element Fishes
    (if (!= _array_element self)
      (set `local.accumulatedDirection` (+ (`KismetMathLibrary.Normal2D` (`/Game/Blueprints/AI/FlockFlish_BP.moveDirection` _array_element)) (`local.accumulatedDirection`)))))
  (return (`KismetMathLibrary.Normal2D` (`local.accumulatedDirection`))))

(fn `calcAvoidanceVector`
  (params (Fishes :type "Array of /Game/Blueprints/AI/FlockFlish_BP Object Reference"))
  (returns (`avoidance Vector` :type "Vector2D Structure"))
  (locals (accumulatedAvoidance :type "Vector2D Structure") (numAvoid :type Integer))
  (for _array_element Fishes
    (if (!= _array_element self)
      (bind _radius (`self.getRadius`))
      (if (< (`KismetMathLibrary.Abs` (`KismetMathLibrary.VSize2D` (- (`/Game/Blueprints/AI/FlockFlish_BP.position` _array_element) (`self.position`)))) (* _radius (`self.minDistance`)))
        (`/Engine/EditorBlueprintResources/StandardMacros.IncrementInt` (`local.numAvoid`)
          (:`  `
            (set `local.accumulatedAvoidance` (+ (`local.accumulatedAvoidance`) (`KismetMathLibrary.Normal2D` (- (`self.position`) (`/Game/Blueprints/AI/FlockFlish_BP.position` _array_element))))))))))
  (return (`KismetMathLibrary.Normal2D` (`local.accumulatedAvoidance`))))

(fn `calcCenterVector`
  (params (Fishes :type "Array of /Game/Blueprints/AI/FlockFlish_BP Object Reference"))
  (returns (centerVec :type "Vector2D Structure"))
  (locals (avgCenter :type "Vector2D Structure"))
  (for _array_element Fishes
    (if (!= _array_element self)
      (set `local.avgCenter` (+ (`/Game/Blueprints/AI/FlockFlish_BP.position` _array_element) (`local.avgCenter`)))))
  (return (`KismetMathLibrary.Normal2D` (- (/ (`local.avgCenter`) (`KismetMathLibrary.Conv_IntToDouble` (`KismetArrayLibrary.Array_Length` Fishes))) (`self.position`)))))

(fn `clacTargetDir`
  (returns (targetDirection :type "Vector2D Structure"))
  (return (`KismetMathLibrary.Normal2D` (- (`/Game/Blueprints/AI/Flock_BP.goalPos` (`self.flock`)) (`self.position`)))))

(fn `getRadius`
  (returns (radius :type "Float (double-precision)"))
  (return (`.SphereRadius` (`KismetSystemLibrary.GetComponentBounds` (`self.Capsule`)))))

(fn `updateDirection`
  (params (deltaTime :type "Float (double-precision)"))
  (set `self.moveDirection` (`KismetMathLibrary.Vector2DInterpTo` (`self.moveDirection`) (`self.targetMoveDirection`) deltaTime (`self.agility`))))

(fn `updateLocation`
  (params (deltaTime :type "Float (double-precision)"))
  ;[1 1 1] Increment the position
  (bind _output_get (set `self.position` (+ (* (* (`KismetMathLibrary.Normal2D` (`self.moveDirection`)) (`self.speed`)) deltaTime) (`self.position`))))
  (bind (_x _y) (`KismetMathLibrary.BreakVector2D` _output_get))
  (bind _worldcoordinates (`/Game/Blueprints/AI/AiPane_BP.getXYZfromUV` (`/Game/Blueprints/AI/Flock_BP.pane` (`self.flock`)) (`KismetMathLibrary.MakeVector2D` _x (`KismetMathLibrary.FClamp` _y 0.0 (`/Game/Blueprints/AI/AiPane_BP.height` (`/Game/Blueprints/AI/Flock_BP.pane` (`self.flock`)))))))
  (`self.K2_SetActorLocation` _worldcoordinates)
  (bind _worldcoordinates_2 (`/Game/Blueprints/AI/AiPane_BP.getXYZfromUV` (`/Game/Blueprints/AI/Flock_BP.pane` (`self.flock`)) (+ (* (* (`KismetMathLibrary.Normal2D` (`self.moveDirection`)) (`self.speed`)) deltaTime) (`self.position`))))
  (`SceneComponent.K2_SetRelativeRotation` (`self.DefaultSceneRoot`) (`KismetMathLibrary.FindLookAtRotation` _worldcoordinates _worldcoordinates_2) false false))

(fn `updateTargetDirection`
  (locals (centerOfFlock :type "Vector2D Structure") (averageDirection :type "Vector2D Structure") (numOfFishes :type Integer) (avoidanceVector :type "Vector2D Structure") (avoidanceCount :type Integer))
  (bind _fishes (`/Game/Blueprints/AI/Flock_BP.fishes` (`self.flock`)))
  ;[1 1 1] Check if we sould update the target Direction
  (if (> (`self.targetUpdatesPerHundret`) (`KismetMathLibrary.RandomFloatInRangeFromStream` 0.0 100.0 (`/Game/Blueprints/AI/Flock_BP.rndStream` (`self.flock`))))
    (bind _centervec (`self.calcCenterVector` _fishes))
    (bind _avgdirection (`self.calcAvgDirection` _fishes))
    (bind _avoidance_vector (`self.calcAvoidanceVector` _fishes))
    (bind _targetdirection (`self.clacTargetDir`))
    (set `self.targetMoveDirection` (`KismetMathLibrary.Normal2D` (+ (* _targetdirection (`self.w_target`)) (+ (* _avoidance_vector (`self.w_separation`)) (+ (* _avgdirection (`self.w_avgDir`)) (* _centervec (`self.w_cohesion`)))))))))

(fn `UserConstructionScript`)