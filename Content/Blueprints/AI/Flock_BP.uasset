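; Flock manager that spawns and tracks a group of FlockFlish_BP fish within a section of a Pane's UV surface.
; On BeginPlay it converts start and end angles and the Pane height into UV bounds, then seeds a time-based random stream.
; Fish spawn at random surface points with a back-reference to the flock and a separately randomized UV Position.
; Each tick, a TargetRashness percent chance moves the GoalPos within those bounds.
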(event `self.ReceiveBeginPlay`
  (bind (_x _y) (`KismetMathLibrary.BreakVector2D` (`self.maxUV`)))
  (bind (_x_2 _y_2) (`KismetMathLibrary.BreakVector2D` (`self.minUV`)))
  (`self.CheckParams`)
  (`self.InitializeRandom`)
  (`self.SpawnFish`)
  (set `self.goalPos` (`KismetMathLibrary.MakeVector2D` (`KismetMathLibrary.RandomFloatInRangeFromStream` _x_2 _x (`self.rndStream`)) (`KismetMathLibrary.RandomFloatInRangeFromStream` _y_2 _y (`self.rndStream`)))))

(event `self.ReceiveTick`
  (params (DeltaSeconds :type "Float (single-precision)"))
  (`self.UpdateTarget`))

(fn `InitializeRandom`
  (bind _seconds (`GameplayStatics.GetAccurateRealTime`))
  (bind _returnvalue (`KismetMathLibrary.MakeRandomStream` _seconds))
  (`KismetMathLibrary.SetRandomStreamSeed` _returnvalue _seconds)
  (set `self.rndStream` _returnvalue))

(fn `ProcessStartParams`)

(fn `UpdateTarget`
  (bind (_x _y) (`KismetMathLibrary.BreakVector2D` (`self.maxUV`)))
  (bind (_x_2 _y_2) (`KismetMathLibrary.BreakVector2D` (`self.minUV`)))
  (if (< (`KismetMathLibrary.RandomFloatInRangeFromStream` 0.0 100.0 (`self.rndStream`)) (`self.targetRashness`))
    (set `self.goalPos` (`KismetMathLibrary.MakeVector2D` (`KismetMathLibrary.RandomFloatInRangeFromStream` _x_2 _x (`self.rndStream`)) (`KismetMathLibrary.RandomFloatInRangeFromStream` _y_2 _y (`self.rndStream`))))))

(fn `UserConstructionScript`)