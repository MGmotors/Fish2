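; AiPane_BP defines a cylindrical pane that maps 2D UV coordinates onto the game's play tube.
; On BeginPlay it takes the tube radius from MyGameInstance and derives MaxU from the circumference.
; Helper functions convert between U and angle, and turn UV into a world position wrapped around the Z axis at Offset, with V as height.
; Each tick it draws the tube as a debug cylinder.
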(event `self.ReceiveBeginPlay`
  (bind _asmy_game_instance (cast `/Game/Blueprints/Game/MyGameInstance` (`GameplayStatics.GetGameInstance`)))
  (set `self.radius` (`/Game/Blueprints/Game/MyGameInstance.playTubeRadius` _asmy_game_instance))
  (set `self.maxU` (* (* (`KismetMathLibrary.GetPI`) 2.0) (`self.radius`))))

(event `self.ReceiveTick`
  (params (DeltaSeconds :type "Float (single-precision)"))
  (`KismetSystemLibrary.DrawDebugCylinder` (`self.offset`) (`KismetMathLibrary.MakeVector` (.x (`self.offset`)) (.y (`self.offset`)) (+ (.z (`self.offset`)) (`self.height`))) (`self.radius`) 64 (struct :`R` 0.37 :`G` 0.046132 :`A` 1.0)))

(fn `getAngleFromU`
  (params (U :type "Float (double-precision)"))
  (returns (AngleDeg :type "Float (double-precision)"))
  (return (* U (/ 360.0 (`self.maxU`)))))

(fn `getUFromAngle`
  (params (angle :type "Float (double-precision)"))
  (returns (u :type "Float (double-precision)"))
  (return (* angle (/ (`self.maxU`) 360.0))))

(fn `getXYZfromUV`
  (params (uv :type "Vector2D Structure"))
  (returns (worldCoordinates :type "Vector Structure"))
  (bind (_x _y) (`KismetMathLibrary.BreakVector2D` uv))
  (bind _angledeg (`self.getAngleFromU` _x))
  (bind (_x_2 _y_2) (`KismetMathLibrary.BreakVector2D` (* (`KismetMathLibrary.Normal2D` (`KismetMathLibrary.MakeVector2D` (`KismetMathLibrary.DegCos` _angledeg) (`KismetMathLibrary.DegSin` _angledeg))) (`self.radius`))))
  (return (+ (`KismetMathLibrary.MakeVector` _x_2 _y_2 _y) (`self.offset`))))

(fn `UserConstructionScript`)