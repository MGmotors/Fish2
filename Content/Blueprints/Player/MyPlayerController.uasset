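; Player controller that gives each player a HUD and handles joining and readying up in the main menu.
; On BeginPlay, it adds a MyHUD widget to the owning player's screen, gated on a controlled pawn check.
; Gamepad Special Right and Enter share one handler: the first press joins, the next readies, tracked by two flags.
; Both actions pass the player's controller ID to MyGameMode's MainMenuWidget.
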(event `self.ReceiveBeginPlay`
  (if (!= (`self.K2_GetPawn` self) null)
    (bind _returnvalue (`|CreateWidget` "/Game/Blueprints/UI/HUD/MyHUD.MyHUD_C" self))
    (`UserWidget.AddToPlayerScreen` _returnvalue 0)))

(event `Key|Gamepad_Special_Right`
  (params (Key :type "Key Structure" :default "AnyKey"))
  (bind _returnvalue (`GameplayStatics.GetGameMode`))
  ;[1 1 1] Input in MainMenu
  (:`Pressed`
    (if (`self.IsJoined`) :!label _label
      (if (not (`self.IsReady`))
        (bind _asmy_game_mode (cast `/Game/Blueprints/Game/MyGameMode` _returnvalue))
        (bind _returnvalue_2 (`GameplayStatics.GetPlayerControllerID` self))
        (`/Game/Blueprints/UI/Menu/MainMenuBP.PlayerReady` (`/Game/Blueprints/Game/MyGameMode.MainMenuWidget` _asmy_game_mode) _returnvalue_2)
        (set `self.IsReady` true))
      (else
        (bind _asmy_game_mode_2 (cast `/Game/Blueprints/Game/MyGameMode` _returnvalue))
        (bind _returnvalue_3 (`GameplayStatics.GetPlayerControllerID` self))
        (`/Game/Blueprints/UI/Menu/MainMenuBP.PlayerJoined` (`/Game/Blueprints/Game/MyGameMode.MainMenuWidget` _asmy_game_mode_2) _returnvalue_3)
        (set `self.IsJoined` true)))))

(event `Key|Enter`
  (params (Key :type "Key Structure" :default "AnyKey"))
  ;[1 1 1] Input in MainMenu
  (:`Pressed`
    (goto _label)))

(fn `UserConstructionScript`)