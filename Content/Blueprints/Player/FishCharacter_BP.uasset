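; Player fish character that swims on the surface of a vertical cylinder around the world origin, eating to grow.
; Tick snaps it to the tube radius, faces it along its velocity and keeps the camera radially outside, looking inward.
; Input moves it around and along the tube, with a rechargeable speed boost.
; Eating flock fish or lower-level players raises level and scale, while hunger builds over time to lower them, using GameInstance tuning.
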(event `self.ReceiveTick`
  (params (DeltaSeconds :type "Float (single-precision)"))
  (bind _charactermovement (`self.CharacterMovement`))
  (bind _charactermovement_2 (`self.CharacterMovement`))
  (bind _returnvalue (`SceneComponent.K2_GetComponentLocation` (`self.CapsuleComponent`)))
  (bind _returnvalue_2 (`SceneComponent.K2_GetComponentLocation` (`self.CapsuleComponent`)))
  (bind _returnvalue_3 (`KismetMathLibrary.MakeVector` (.x _returnvalue_2) (.y _returnvalue_2)))
  (bind _returnvalue_4 (+ (* (`KismetMathLibrary.Normal` (`KismetMathLibrary.MakeVector` (.x (`SceneComponent.K2_GetComponentLocation` (`self.CapsuleComponent`))) (.y (`SceneComponent.K2_GetComponentLocation` (`self.CapsuleComponent`))))) (`/Game/Blueprints/Game/MyGameInstance.playTubeRadius` (`self.gameInstance`))) (`KismetMathLibrary.MakeVector` 0.0 0.0 (.z (`SceneComponent.K2_GetComponentLocation` (`self.CapsuleComponent`))))))
  ;[1 1 1] Correct Position
  (`SceneComponent.K2_SetWorldLocation` (`self.CapsuleComponent`) _returnvalue_4 false false)
  ;[1 1 1] CorrectRotation
  (bind _returnvalue_5 (`PrimitiveComponent.GetPhysicsLinearVelocity` (`self.CapsuleComponent`) "None"))
  (if (> (`KismetMathLibrary.VSize` _returnvalue_5) 0.2)
    (bind _output_get (set `self.lastDirectionNotNull` _returnvalue_5)))
  (`SceneComponent.K2_SetRelativeRotation` (`self.CapsuleComponent`) (`KismetMathLibrary.FindLookAtRotation` _returnvalue_4 (+ _output_get _returnvalue_4)) false false)
  ;[1 1 1] Set Camera Location
  (set `self.cameraFromPlayerDirection` _returnvalue_3)
  (`SceneComponent.K2_SetWorldLocation` (`self.Camera`) (+ _returnvalue_2 (* (`KismetMathLibrary.Normal` _returnvalue_3) (`/Game/Blueprints/Game/MyGameInstance.cameraFromPlayerDistance` (`self.gameInstance`)))) false false)
  ;[1 1 1] Look towards the center
  (`SceneComponent.K2_SetWorldRotation` (`self.Camera`) (`KismetMathLibrary.FindLookAtRotation` (`KismetMathLibrary.MakeVector` (.x _returnvalue) (.y _returnvalue) (.z _returnvalue)) (`KismetMathLibrary.MakeVector` 0.0 0.0 (.z _returnvalue))) false false)
  ;[1 1 1] Boost
  (if (`self.IsBoosting`)
    (bind _output_get_2 (set `self.CurrentBoost` (- (`self.CurrentBoost`) (* DeltaSeconds (`/Game/Blueprints/Game/MyGameInstance.BoostDecreasePerSec` (`self.gameInstance`))))))
    (if (> _output_get_2 0.0)
      (set `CharacterMovementComponent.MaxSwimSpeed` 5000.0 _charactermovement)
      (set `CharacterMovementComponent.MaxAcceleration` 5000.0 _charactermovement)
      (else
        (set `self.IsBoosting` false :!label _label)
        (set `CharacterMovementComponent.MaxSwimSpeed` 1000.0 _charactermovement_2 :!label _label_2)
        (set `CharacterMovementComponent.MaxAcceleration` 1000.0 _charactermovement_2)))
    (else
      (`self.increaseBoost` DeltaSeconds)
      (goto _label_2)))
  (`self.increaseHunger` DeltaSeconds)
  ;[1 1 1] look to the right in the beginning
  (if (< (`KismetMathLibrary.VSize` (`self.lastDirectionNotNull`)) 0.1)
    (set `self.lastDirectionNotNull` (`KismetMathLibrary.GetForwardVector` (`KismetMathLibrary.Conv_VectorToRotator` (`SceneComponent.K2_GetComponentLocation` (`self.CapsuleComponent`)))))))

(event `InputAction|Boost`
  (params (Key :type "Key Structure" :default "AnyKey"))
  ;[1 1 1] Boost
  (:`Pressed`
    (if (> (`self.CurrentBoost`) 0.0)
      (set `self.IsBoosting` true)
      (else
        (goto _label))))
  (:`Released`
    (goto _label)))

(event `InputAxis|Right_Left`
  (params (AxisValue :type "Float (single-precision)"))
  ;[1 1 1] Left/Right Movement
  (`self.AddMovementInput` (`KismetMathLibrary.GetRightVector` (`KismetMathLibrary.Conv_VectorToRotator` (`SceneComponent.K2_GetComponentLocation` (`self.CapsuleComponent`)))) (* AxisValue (`/Game/Blueprints/Game/MyGameInstance.playerSpeed` (`self.gameInstance`))) true))

(event `InputAxis|top_bot`
  (params (AxisValue :type "Float (single-precision)"))
  (`self.AddMovementInput` (0.0 0.0 1.0) (* AxisValue (`/Game/Blueprints/Game/MyGameInstance.playerSpeed` (`self.gameInstance`))) true))

(event `self.ReceiveActorBeginOverlap`
  (params (OtherActor :type "Actor Object Reference"))
  (`|ExecutionSequence`
    (:`then_0`
      (bind _asflock_flish_bp (cast `/Game/Blueprints/AI/FlockFlish_BP` OtherActor))
      (`/Game/Blueprints/AI/FlockFlish_BP.Eaten` _asflock_flish_bp)
      ;[1 1 1] Growing
      (set `self.currentHunger` 0.0)
      (if (< (`self.currentLevel`) 100.0) :!label _label_3
        (`/Engine/EditorBlueprintResources/StandardMacros.IncrementFloat` (`self.currentLevel`)
          (:`  `
            (`self.setScaleBasedOnLevel`)))))
    (:`then_1`
      ;[1 1 1] Player vs Player
      (bind _asfish_character_bp (cast `/Game/Blueprints/Player/FishCharacter_BP` OtherActor))
      (if (> (`self.currentLevel`) (`/Game/Blueprints/Player/FishCharacter_BP.currentLevel` _asfish_character_bp))
        (`self.Eaten` _asfish_character_bp)
        (goto _label_3)))))

(event `self.ReceiveBeginPlay`
  (set `self.baseScale` (`self.GetActorScale3D`))
  (bind _asmy_game_instance (cast `/Game/Blueprints/Game/MyGameInstance` (`GameplayStatics.GetGameInstance`)))
  (set `self.gameInstance` _asmy_game_instance))

(event `self.ReceiveEndPlay`
  (params (EndPlayReason :type "EEndPlayReason Enum" :default "Destroyed")))

(event `Eaten`
  (`self.K2_DestroyActor`))

(fn `AngleBetweenVectors`
  (params (A :type "Vector Structure") (B :type "Vector Structure"))
  (returns (angle :type "Float (double-precision)"))
  (return (`KismetMathLibrary.DegAcos` (`KismetMathLibrary.Dot_VectorVector` (`KismetMathLibrary.Normal` A) (`KismetMathLibrary.Normal` B)))))

(fn `increaseBoost`
  (params (deltaTime :type "Float (double-precision)"))
  (if (< (`self.CurrentBoost`) 1.0)
    (set `self.CurrentBoost` (`KismetMathLibrary.FClamp` (+ (`self.CurrentBoost`) (* deltaTime (`/Game/Blueprints/Game/MyGameInstance.BoostInceasePerSec` (`self.gameInstance`))))))))

(fn `increaseHunger`
  (params (deltaTime :type "Float (double-precision)"))
  (set `self.currentHunger` (+ (* (`/Game/Blueprints/Game/MyGameInstance.HungerIncreasePerSec` (`self.gameInstance`)) deltaTime) (`self.currentHunger`)))
  (if (> (`self.currentHunger`) 1.0)
    (if (> (`self.currentLevel`) 1.0)
      (`/Engine/EditorBlueprintResources/StandardMacros.DecrementFloat` (`self.currentLevel`)
        (:`  `
          (set `self.currentHunger` 0.0)
          (`self.setScaleBasedOnLevel`))))))

(fn `setScaleBasedOnLevel`
  (`self.SetActorScale3D` (+ (`self.baseScale`) (* (`self.currentLevel`) (`/Game/Blueprints/Game/MyGameInstance.ScalePerLevel` (`self.gameInstance`))))))

(fn `UserConstructionScript`)